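; BP_SoulActor is a soul actor that homes in on player character 0.
; Each Tick moves it straight toward the player at a speed set by Velocity, without sweep, then passes its new location to the Niagara component as TailLocation.
; An unconnected Timeline movement branch and an empty RandomMove function are present but do nothing.
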(event EventBeginPlay)

(event EventTick
  (params (DeltaSeconds :type Float%20%28single-precision%29))
  (Transformation|SetActorLocation (+ (Transformation|GetActorLocation) (* (* (Math|Vector|Normalize (- (Transformation|GetActorLocation (Game|GetPlayerCharacter 0)) (Transformation|GetActorLocation))) (Variables|Default|GetVelocity)) DeltaSeconds)) false false)
  (Class|NiagaraComponent|SetNiagaraVariableVec3 (Variables|Default|GetNiagara) "TailLocation" (Transformation|GetActorLocation)))

(fn ConstructionScript)

(fn RandomMove)