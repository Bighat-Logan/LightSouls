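; BP_YakuEnemy is an enemy Blueprint that keeps its health bar in sync with its health.
; On health change it runs the parent handler, then reads current and max health from the ability system's LsCommonAttributeSet.
; If the LsHealthBarActor's widget implements HealthBarInterface, it sends the health ratio to the widget and the raw values to the actor.
; Impact force changes only print a debug string, and construction defers to the parent.
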(event EventOnImpactForceChange
  (params (ImpactForce :type ELsImpactForce%20Enum :default "None") (ImpactForceVector :type Vector :default "0, 0, 0") (HitInfo :type Hit%20Result%20Structure%20%28by%20ref%29) (ImpactTags :type Gameplay%20Tag%20Container%20Structure%20%28by%20ref%29) (InstigatorCharacter :type Ls%20Character%20Base%20Object%20Reference) (ImpactCauser :type Actor%20Object%20Reference))
  (Development|PrintString "A"))

(event EventOnHealthChange
  (params (DamageAmount :type Float%20%28single-precision%29) (HitInfo :type Hit%20Result%20Structure%20%28by%20ref%29) (DamageTags :type Gameplay%20Tag%20Container%20Structure%20%28by%20ref%29) (InstigatorCharacter :type Ls%20Character%20Base%20Object%20Reference) (DamageCauser :type Actor%20Object%20Reference))
  (bind _lshealthbaractor (Variables|Default|GetLsHealthBarActor))
  (bind _returnvalue (Class|LsHealthBarActorComponent|GetHealthBarWidgetComponent _lshealthbaractor))
  (bind _returnvalue_2 (UserInterface|GetWidget _returnvalue))
  (|CallParentFunction DamageAmount HitInfo DamageTags InstigatorCharacter DamageCauser)
  (bind _returnvalue_3 (GameplayAttributes|GetAttributeSet (Ability|GetAbilitySystemComponent 0) "/Script/LightSouls.LsCommonAttributeSet"))
  (bind _asls_common_attribute_set (Utilities|Casting|CastToLsCommonAttributeSet _returnvalue_3))
  (if (Utilities|DoesObjectImplementInterface _returnvalue_2 "/Script/LightSouls.HealthBarInterface")
    (Class|HealthBarInterface|ChangeHealth(Message) _returnvalue_2 (/ (.currentvalue (Variables|/Script/LightSouls.LsCommonAttributeSet|GetHealth _asls_common_attribute_set)) (.currentvalue (Variables|/Script/LightSouls.LsCommonAttributeSet|GetMaxHealth _asls_common_attribute_set))))
    (Class|LsHealthBarActorComponent|UpdateHealthBar (Variables|Default|GetLsHealthBarActor) (.currentvalue (Variables|/Script/LightSouls.LsCommonAttributeSet|GetHealth _asls_common_attribute_set)) (.currentvalue (Variables|/Script/LightSouls.LsCommonAttributeSet|GetMaxHealth _asls_common_attribute_set)))))

(fn ConstructionScript
  (|CallParentFunction))