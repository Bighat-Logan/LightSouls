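; Enemy Blueprint with a camera-facing health bar, hit reactions and an effect-driven death.
; Health changes feed the GAS Health/MaxHealth ratio to the bar widget.
; Impact force drives a head hit in the anim Blueprint, blended by a timeline, and damage plays a sound.
; A death montage notify starts Niagara and a timeline animating "Mask" on mesh materials and particles, deferring parent death logic until the particles finish.
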(event Custom|OnSystemFinished_Event
  (params (PSystem :type Niagara%20Component%20Object%20Reference))
  (|CallParentFunction (stale EventOnDeath DamageAmount) (stale EventOnDeath DamageTags) (stale EventOnDeath InstigatorCharacter) (stale EventOnDeath DamageCauser)))

(event EventOnImpactForceChange
  (params (ImpactForce :type ELsImpactForce%20Enum :default "None") (ImpactForceVector :type Vector :default "0, 0, 0") (HitInfo :type Hit%20Result%20Structure%20%28by%20ref%29) (ImpactTags :type Gameplay%20Tag%20Container%20Structure%20%28by%20ref%29) (InstigatorCharacter :type Ls%20Character%20Base%20Object%20Reference) (ImpactCauser :type Actor%20Object%20Reference))
  (if (not (Variables|Default|GetInHitTrigger))
    (bind _asabp_enemy_base (Utilities|Casting|CastToABP_EnemyBase (Components|SkeletalMesh|GetAnimInstance (Variables|Character|GetMesh))))
    (bind _returnvalue (Class|LsUtilityLibrary|NormalizeVector ImpactForceVector))
    (Default|SetHitParam _asabp_enemy_base true "head" 0.3 _returnvalue)
    (bind _hitalpha (Timeline|Timeline PlayFromStart)
      (:Update
        (Default|SetAlpha _asabp_enemy_base _hitalpha)))))

(event EventBeginPlay
  (Class|LsUtilityLibrary|EnsureSkeletalMeshMaterialsAreDynamic (Variables|Character|GetMesh))
  (Class|LsUtilityLibrary|SetScalarParameteronSkeletalMeshMIDs (Variables|Character|GetMesh) "Mask" 1.0))

(event EventOnHealthChange
  (params (DamageAmount :type Float%20%28single-precision%29) (HitInfo :type Hit%20Result%20Structure%20%28by%20ref%29) (DamageTags :type Gameplay%20Tag%20Container%20Structure%20%28by%20ref%29) (InstigatorCharacter :type Ls%20Character%20Base%20Object%20Reference) (DamageCauser :type Actor%20Object%20Reference))
  (|CallParentFunction DamageAmount HitInfo DamageTags InstigatorCharacter DamageCauser)
  (bind _aswbg_health_bar (Utilities|Casting|CastToWBG_HealthBar (UserInterface|GetWidget (Variables|Default|GetHealthBar))))
  (bind _returnvalue (GameplayAttributes|GetAttributeSet (Ability|GetAbilitySystemComponent 0) "/Script/LightSouls.LsCommonAttributeSet"))
  (bind _asls_common_attribute_set (Utilities|Casting|CastToLsCommonAttributeSet _returnvalue))
  (Class|HealthBarInterface|ChangeHealth _aswbg_health_bar (/ (.currentvalue (Variables|/Script/LightSouls.LsCommonAttributeSet|GetHealth _asls_common_attribute_set)) (.currentvalue (Variables|/Script/LightSouls.LsCommonAttributeSet|GetMaxHealth _asls_common_attribute_set)))))

(event EventOnDamaged
  (params (DamageAmount :type Float%20%28single-precision%29) (HitInfo :type Hit%20Result%20Structure%20%28by%20ref%29) (DamageTags :type Gameplay%20Tag%20Container%20Structure%20%28by%20ref%29) (InstigatorCharacter :type Ls%20Character%20Base%20Object%20Reference) (DamageCauser :type Actor%20Object%20Reference))
  (Audio|PlaySound2D "/Game/Game/Sound/BeHit.BeHit" 1.0 1.0 0.0 0 0))

(event EventTick
  (params (DeltaSeconds :type Float%20%28single-precision%29))
  (bind _healthbar (Variables|Default|GetHealthBar))
  (Transformation|SetWorldRotation _healthbar (Math|Rotator|FindLookatRotation (Transformation|GetWorldLocation _healthbar) (Transformation|GetWorldLocation (Variables|/Script/Engine.Actor|GetRootComponent (Game|GetPlayerCameraManager 0)))) false false))

(event EventOnDeath
  (params (DamageAmount :type Float%20%28single-precision%29) (DamageTags :type Gameplay%20Tag%20Container%20Structure%20%28by%20ref%29) (InstigatorCharacter :type Ls%20Character%20Base%20Object%20Reference) (DamageCauser :type Actor%20Object%20Reference))
  (Animation|Montage|PlayMontage (Variables|Character|GetMesh) (Variables|Default|GetDeathMontage)
    (:OnNotifyBegin
      (Components|Activation|Activate (Variables|Default|GetNiagara) false)
      (bind _mask (Timeline|Timeline_0 PlayFromStart)
        (:Update
          (Class|LsUtilityLibrary|SetScalarParameteronSkeletalMeshMIDs (Variables|Character|GetMesh) "Mask" _mask)
          (Niagara|SetNiagaraVariable(Float) (Variables|Default|GetNiagara) "Mask" _mask)
          (EventDispatchers|AssignOnSystemFinished (Variables|Default|GetNiagara) (delegate Custom|OnSystemFinished_Event)))))))

(fn ConstructionScript
  (|CallParentFunction))