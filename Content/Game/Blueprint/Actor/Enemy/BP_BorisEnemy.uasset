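; Enemy actor for Boris, with a floating health bar driven by the Gameplay Ability System's common attribute set.
; Tick rotates the health bar to face the player camera.
; Each health change pushes the health-to-max ratio to the bar widget and raises the mesh materials' FadeOut parameter by a fixed step, regardless of the amount changed.
; The impact-force event only prints a debug string, and a health debug printout is left unconnected.
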(event EventTick
  (params (DeltaSeconds :type Float%20%28single-precision%29))
  (bind _healthbar (Variables|Default|GetHealthBar))
  (Transformation|SetWorldRotation _healthbar (Math|Rotator|FindLookatRotation (Transformation|GetWorldLocation _healthbar) (Transformation|GetWorldLocation (Variables|/Script/Engine.Actor|GetRootComponent (Game|GetPlayerCameraManager 0)))) false false))

(event EventOnHealthChange
  (params (DamageAmount :type Float%20%28single-precision%29) (HitInfo :type Hit%20Result%20Structure%20%28by%20ref%29) (DamageTags :type Gameplay%20Tag%20Container%20Structure%20%28by%20ref%29) (InstigatorCharacter :type Ls%20Character%20Base%20Object%20Reference) (DamageCauser :type Actor%20Object%20Reference))
  (bind _aswbg_health_bar (Utilities|Casting|CastToWBG_HealthBar (UserInterface|GetWidget (Variables|Default|GetHealthBar))))
  (bind _returnvalue (GameplayAttributes|GetAttributeSet (Ability|GetAbilitySystemComponent 0) "/Script/LightSouls.LsCommonAttributeSet"))
  (bind _asls_common_attribute_set (Utilities|Casting|CastToLsCommonAttributeSet _returnvalue))
  (Default|ChangeHealth _aswbg_health_bar (/ (.currentvalue (Variables|/Script/LightSouls.LsCommonAttributeSet|GetHealth _asls_common_attribute_set)) (.currentvalue (Variables|/Script/LightSouls.LsCommonAttributeSet|GetMaxHealth _asls_common_attribute_set))))
  (Variables|Default|SetFadeOut (+ (Variables|Default|GetFadeOut) 0.1))
  (Class|LsUtilityLibrary|SetScalarParameteronSkeletalMeshMIDs (Variables|Character|GetMesh) "FadeOut" (Variables|Default|GetFadeOut)))

(event EventOnImpactForceChange
  (params (ImpactForce :type ELsImpactForce%20Enum :default "None") (ImpactForceVector :type Vector :default "0, 0, 0") (HitInfo :type Hit%20Result%20Structure%20%28by%20ref%29) (ImpactTags :type Gameplay%20Tag%20Container%20Structure%20%28by%20ref%29) (InstigatorCharacter :type Ls%20Character%20Base%20Object%20Reference) (ImpactCauser :type Actor%20Object%20Reference))
  (Development|PrintString "Hello"))

(fn ConstructionScript
  (|CallParentFunction))