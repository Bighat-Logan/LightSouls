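; Base enemy Blueprint that reacts to AI perception and handles health-driven death through the Ability System.
; Perception updates are checked per sense by matching stimuli classes: sight sets the AIC_Enemy_Base controller to attacking, while hearing and damage only print debug strings.
; Health changes trigger death handling when the LsCommonAttributeSet Health reaches zero, and the death event destroys the actor after a short delay.
; It also makes mesh materials dynamic on BeginPlay and exposes its attack volume array.
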(event OnPerceptionUpdated(AIPerception)
  (params (UpdatedActors :type Array%20of%20Actor%20Object%20References))
  (for _array_element UpdatedActors
    (Utilities|FlowControl|Sequence
      (:then_0
        (bind _sensed (CallFunction|CanSenceActor _array_element "NewEnumerator1"))
        (if _sensed
          (CallFunction|HandleSensedSight _array_element)))
      (:then_1
        (bind _sensed_2 (CallFunction|CanSenceActor _array_element "NewEnumerator2"))
        (if _sensed_2
          (Development|PrintString "Hearing sense")))
      (:then_2
        (bind _sensed_3 (CallFunction|CanSenceActor _array_element "NewEnumerator3"))
        (if _sensed_3
          (Development|PrintString "Damage sense"))))))

(event EventBeginPlay
  (Class|LsUtilityLibrary|EnsureSkeletalMeshMaterialsAreDynamic (Variables|Character|GetMesh)))

(event EventOnHealthChange
  (params (DamageAmount :type Float%20%28single-precision%29) (HitInfo :type Hit%20Result%20Structure%20%28by%20ref%29) (DamageTags :type Gameplay%20Tag%20Container%20Structure%20%28by%20ref%29) (InstigatorCharacter :type Ls%20Character%20Base%20Object%20Reference) (DamageCauser :type Actor%20Object%20Reference))
  (bind _returnvalue (GameplayAttributes|GetAttributeSet (Ability|GetAbilitySystemComponent 0) "/Script/LightSouls.LsCommonAttributeSet"))
  (bind _asls_common_attribute_set (Utilities|Casting|CastToLsCommonAttributeSet _returnvalue))
  (if (<= (.currentvalue (Variables|/Script/LightSouls.LsCommonAttributeSet|GetHealth _asls_common_attribute_set)) 0.0)
    (Class|LsCharacterBase|HandleDeath DamageAmount DamageTags InstigatorCharacter DamageCauser)))

(event EventOnDeath
  (params (DamageAmount :type Float%20%28single-precision%29) (DamageTags :type Gameplay%20Tag%20Container%20Structure%20%28by%20ref%29) (InstigatorCharacter :type Ls%20Character%20Base%20Object%20Reference) (DamageCauser :type Actor%20Object%20Reference))
  (Utilities|FlowControl|Delay 0.2)
  (Actor|DestroyActor))

(fn ConstructionScript)

(fn CanSenceActor
  (params (Actor :type Actor%20Object%20Reference) (Sence :type E_AIPerceptionType%20Enum :default "NewEnumerator0"))
  (bind _info (Class|AIPerceptionComponent|GetActorsPerception (Variables|Default|GetAIPerception) Actor))
  (for _array_element (.LastSensedStimuli (Utilities|Struct|BreakActorPerceptionBlueprintInfo _info))
    (bind _returnvalue (Class|AIPerceptionSystem|GetSenseClassforStimulus _array_element))
    (if (== _returnvalue (Utilities|Select :Index Sence :NewEnumerator0 0 :NewEnumerator1 "/Script/AIModule.AISense_Sight" :NewEnumerator2 "/Script/AIModule.AISense_Hearing" :NewEnumerator3 "/Script/AIModule.AISense_Damage"))
      (return (.bSuccessfullySensed (Utilities|Struct|BreakAIStimulus _array_element)) _array_element))))

(fn HandleSensedSight
  (params (Actor :type Actor%20Object%20Reference))
  (bind _asaic_enemy_base (Utilities|Casting|CastToAIC_Enemy_Base (Pawn|GetController)))
  (Default|SetStateasAttacking _asaic_enemy_base Actor))

(fn GetAllAttackVolume
  (return (Variables|Default|GetAttackVolumeArray)))