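; Player character Blueprint that carries a sword and turns attack input into Gameplay Ability System attacks.
; On BeginPlay it spawns the weapon actor and attaches it to the mesh's blade socket.
; Attack input, unless blocked by a gameplay tag, has the combo component evaluate combat state for a short attack and activates the returned ability class.
; Debug prints include a BeginPlay test string and owned gameplay tags every Tick.
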(event Input|EnhancedActionEvents|EnhancedInputActionIA_Attack
  (params (ActionValue :type Boolean) (ElapsedSeconds :type Float%20%28double-precision%29) (TriggeredSeconds :type Float%20%28double-precision%29) (InputAction :type Input%20Action%20Object%20Reference :default "/Game/Game/Input/IA_Attack.IA_Attack"))
  (if (not (GameplayTags|HasMatchingGameplayTag (Ability|GetAbilitySystemComponent 0) "(TagName=\"InputState.BlockInput\")"))
    (bind _returnvalue (Class|LsComboActorComponent|EvaluateCombatState (Variables|Default|GetComboComponent) self "IA_Attack_Short"))
    (Abilities|TryActivateAbilitybyClass (Ability|GetAbilitySystemComponent 0) _returnvalue true)))

(event EventBeginPlay
  (bind _returnvalue (Game|SpawnActorfromClass (Variables|Default|GetNewVar) (Transformation|GetActorTransform) "Undefined" "MultiplyWithRoot" 0 0))
  (bind _output_get (Variables|Default|SetSwordActor _returnvalue))
  (Transformation|AttachComponentToComponent _output_get (Variables|Character|GetMesh) "Weapon_BladeSocket" "SnapToTarget" "KeepRelative" "KeepRelative" false)
  (Development|PrintString "Test"))

(event EventTick
  (params (DeltaSeconds :type Float%20%28single-precision%29))
  (Development|PrintString (GameplayTags|GetDebugStringfromGameplayTagContainer (GameplayTags|GetOwnedGameplayTags (Ability|GetAbilitySystemComponent 0) :!class /Script/GameplayTags.GameplayTagAssetInterface)) false))

(fn ConstructionScript)