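; Player controller that sets up gameplay input and handles opening and closing the in-game menu.
; On BeginPlay it hides the cursor, clears the PlayerState.InOptionMenu tag from the game instance's global tags and switches to game-only input.
; The option action event fetches the InGameMenu CommonUI activatable stack from the widget stack subsystem and passes it to ToggleInGameMenu.
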(event EventHandleOptionAction
  (bind _ascommon_activatable_widget_stack (Utilities|Casting|CastToCommonActivatableWidgetStack (Class|LsWidgetStackSubsystem|GetWidgetStack (Subsystems|GetLsWidgetStackSubsystem) "(TagName=\"UI.WidgetStack.InGameMenu\")")))
  (Class|LsUtilityLibrary|ToggleinGameMenu _ascommon_activatable_widget_stack))

(event EventBeginPlay
  (Variables|Default|SetbShowMouseCursor false)
  (GameplayTags|RemoveGameplayTag (Variables|/Script/LightSouls.LsGameInstance|GetGlobalGameTags (Class|LsUtilityLibrary|GetLsGameInstance self)) "(TagName=\"PlayerState.InOptionMenu\")" :!class /Script/GameplayTags.BlueprintGameplayTagLibrary)
  (Input|SetInputModeGameOnly self false))

(fn ConstructionScript)